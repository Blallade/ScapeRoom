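; CodeDevice is an interactable device that displays blinking screen text and opens a code device UI.
; From BeginPlay, an endless Delay loop switches ScreenText between two values every half second.
; InteractiveEvent finds the first top-level CodeDeciveUI widget through GetAllWidgetsOfClass and calls ShowCodeDevice on it, passing along the event's Object.
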(event `self.ReceiveBeginPlay`
  (bind _screentext (`self.ScreenText`))
  (`TextRenderComponent.K2_SetText` _screentext (`self.Value`) :!label _label)
  (`KismetSystemLibrary.Delay` 0.5)
  (`TextRenderComponent.K2_SetText` _screentext (`self.Value_0`))
  (`KismetSystemLibrary.Delay` 0.5)
  (goto _label))

(event `/Game/Blueprints/InteractiveEvent.InteractiveEvent`
  (params (Object :type "Actor Object Reference"))
  (bind _foundwidgets (`WidgetBlueprintLibrary.GetAllWidgetsOfClass` "/Game/Blueprints/UI/CodeDeciveUI.CodeDeciveUI_C"))
  (`/Game/Blueprints/UI/CodeDeciveUI.ShowCodeDevice` (`|GetArrayItem` _foundwidgets) Object))

(fn `UserConstructionScript`)