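; ObtainableObject is a Blueprint for an interactable object that passes confirm and back key presses to the player UI.
; CanPress? turns input on the object on or off for the first player controller.
; The Continue key calls the PlayerUI confirm, back and pick handlers together, while BackKey calls its back handler, with the widget found by class lookup.
; DisableController sets the character's Targetting flag and switches to cursor-driven Game and UI input.
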(event `CanPress?`
  (params (`IsActive?` :type Boolean))
  (bind _returnvalue (`GameplayStatics.GetPlayerController` 0))
  ;[0.7622 0.4247 1] Enables the input on the specific object
  (if `IsActive?`
    (`self.EnableInput` _returnvalue)
    (else
      (`self.DisableInput` _returnvalue))))

(event `InputAction|Continue`
  (params (Key :type "Key Structure"))
  ;[1 0.3412 0.3412] "E" input in the specific object
  (:`Pressed`
    (bind _foundwidgets (`WidgetBlueprintLibrary.GetAllWidgetsOfClass` "/Game/Blueprints/UI/PlayerUI.PlayerUI_C"))
    (bind _output (`|GetArrayItem` _foundwidgets))
    (`/Game/Blueprints/UI/PlayerUI.PressEToConfirm` _output)
    (`/Game/Blueprints/UI/PlayerUI.PressEToBack` _output)
    (`/Game/Blueprints/UI/PlayerUI.PressEToPick` _output)))

(event `InputAction|BackKey`
  (params (Key :type "Key Structure"))
  ;[1 0.3412 0.3412] Back key event
  (:`Pressed`
    (bind _foundwidgets (`WidgetBlueprintLibrary.GetAllWidgetsOfClass` "/Game/Blueprints/UI/PlayerUI.PlayerUI_C"))
    (`/Game/Blueprints/UI/PlayerUI.PressBackKey` (`|GetArrayItem` _foundwidgets))))

(fn `DisableController`
  (params (WidgetToFocus :type "Widget Object Reference"))
  (bind _returnvalue (`GameplayStatics.GetPlayerController` 0))
  (set `/Game/Blueprints/FirstPersonCharacter.Targetting` true (cast `/Game/Blueprints/FirstPersonCharacter` (`GameplayStatics.GetPlayerPawn` 0) :!pure true))
  (`WidgetBlueprintLibrary.SetInputMode_GameAndUIEx` _returnvalue WidgetToFocus)
  (set `PlayerController.bShowMouseCursor` true _returnvalue))

(fn `UserConstructionScript`
  (`parent.UserConstructionScript`))