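; Interactive actor that toggles the player character between normal and 20x scale.
; Capsule overlap shows an interact prompt on PlayerUI; interacting locks input, plays the SizeChangerUI effect and sound, then after a delay tilts the view and sets fixed height and scale.
; The first shrink hands input to this actor until Continue hides the SizeChangerUI message.
; Capsule collision stays off during each change to block retriggering.
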(event `InputAction|Continue`
  (params (Key :type "Key Structure"))
  (bind _returnvalue (`GameplayStatics.GetPlayerController` 0))
  ;[0.4108 0.3325 1] Changes the size of the player
  (:`Pressed`
    (`self.DisableInput` _returnvalue)
    (`self.EnableInput` (stale `/Game/Blueprints/InteractiveEvent.InteractiveEvent` _returnvalue_3) _returnvalue)
    (`/Game/Blueprints/UI/SizeChangerUI.ShowMessage` (`|GetArrayItem` (stale `/Game/Blueprints/InteractiveEvent.InteractiveEvent` _foundwidgets)) false)
    (set `self.IsFirstUse?` false)
    (`PrimitiveComponent.SetCollisionEnabled` (`self.Capsule`) "QueryOnly")))

(event `/Game/Blueprints/InteractiveEvent.InteractiveEvent`
  (params (Object :type "Actor Object Reference"))
  (bind _returnvalue (`GameplayStatics.GetPlayerController` 0))
  (bind _returnvalue_2 (`GameplayStatics.GetPlayerController` 0))
  (bind _asfirst_person_character (cast `/Game/Blueprints/FirstPersonCharacter` (`GameplayStatics.GetPlayerCharacter` 0) :!pure true))
  (bind (_returnvalue_x _returnvalue_y) (`KismetMathLibrary.BreakVector` (`self.K2_GetActorLocation` _asfirst_person_character)))
  (bind (_returnvalue_x_2 _returnvalue_y_2) (`KismetMathLibrary.BreakVector` (`self.K2_GetActorLocation` _asfirst_person_character)))
  (bind (_returnvalue_roll _returnvalue_pitch _returnvalue_yaw) (`KismetMathLibrary.BreakRotator` (`Pawn.GetControlRotation` _asfirst_person_character)))
  ;[0.4108 0.3325 1] Changes the size of the player
  (`PrimitiveComponent.SetCollisionEnabled` (`self.Capsule`) "NoCollision")
  (bind _foundwidgets (`WidgetBlueprintLibrary.GetAllWidgetsOfClass` "/Game/Blueprints/UI/SizeChangerUI.SizeChangerUI_C"))
  (`/Game/Blueprints/UI/SizeChangerUI.ChangingSize` (`|GetArrayItem` _foundwidgets))
  (set `PlayerController.bShowMouseCursor` false _returnvalue)
  (`GameplayStatics.PlaySound2D` "/Game/Audio/SoundFx/Portal.Portal" 0.3 1.5 0.0 null null)
  (bind _returnvalue_3 (`GameplayStatics.GetActorOfClass` "/Game/Blueprints/FirstPersonCharacter.FirstPersonCharacter_C"))
  (`self.DisableInput` _returnvalue_3 _returnvalue)
  (`KismetSystemLibrary.Delay` 2.0)
  (`Controller.SetControlRotation` _returnvalue (`KismetMathLibrary.MakeRotator` _returnvalue_roll (+ _returnvalue_pitch 45.0) _returnvalue_yaw))
  ;;[1 0 0] Choose between big or small to change the size.
  (if (`self.IsBig?`)
    (`self.K2_SetActorTransform` _asfirst_person_character (`KismetMathLibrary.MakeTransform` (`KismetMathLibrary.MakeVector` _returnvalue_x_2 _returnvalue_y_2 148.0)) false false)
    (`/Game/Blueprints/FirstPersonCharacter.ChangeSize` _asfirst_person_character true)
    (bind _foundwidgets_2 (`WidgetBlueprintLibrary.GetAllWidgetsOfClass` "/Game/Blueprints/UI/PlayerUI.PlayerUI_C"))
    (`/Game/Blueprints/UI/PlayerUI.Return` (`|GetArrayItem` _foundwidgets_2) Object)
    (set `self.IsBig?` false)
    ;;[1 0 0] Detects if it is the first time he changes his size.
    (if (`self.IsFirstUse?`)
      (`self.EnableInput` _returnvalue_2)
      (else
        (`self.EnableInput` _returnvalue_3 _returnvalue_2)
        (`PrimitiveComponent.SetCollisionEnabled` (`self.Capsule`) "QueryOnly")))
    (else
      (`self.K2_SetActorTransform` _asfirst_person_character (`KismetMathLibrary.MakeTransform` (`KismetMathLibrary.MakeVector` _returnvalue_x _returnvalue_y 1970.0) (struct) (20.0 20.0 20.0)) false false)
      (`/Game/Blueprints/FirstPersonCharacter.ChangeSize` _asfirst_person_character false)
      (bind _foundwidgets_3 (`WidgetBlueprintLibrary.GetAllWidgetsOfClass` "/Game/Blueprints/UI/PlayerUI.PlayerUI_C"))
      (`/Game/Blueprints/UI/PlayerUI.Return` (`|GetArrayItem` _foundwidgets_3) Object)
      (set `self.IsBig?` true)
      (`self.EnableInput` _returnvalue_3 (`GameplayStatics.GetPlayerController` 0))
      (`PrimitiveComponent.SetCollisionEnabled` (`self.Capsule`) "QueryOnly"))))

(event `self.Capsule.OnComponentBeginOverlap`
  (params (OverlappedComponent :type "PrimitiveComponent Object Reference") (OtherActor :type "Actor Object Reference") (OtherComp :type "PrimitiveComponent Object Reference") (OtherBodyIndex :type Integer) (bFromSweep :type Boolean) (SweepResult :type "HitResult Structure (by ref)"))
  ;[0.5569 0.749 1] Specific collision for this event object
  (cast `/Game/Blueprints/FirstPersonCharacter` OtherActor)
  (bind _foundwidgets (`WidgetBlueprintLibrary.GetAllWidgetsOfClass` "/Game/Blueprints/UI/PlayerUI.PlayerUI_C"))
  (`/Game/Blueprints/UI/PlayerUI.ShowInteractAdvice` (`|GetArrayItem` _foundwidgets) true)
  (set `self.isOverlapping?` true))

(event `self.Capsule.OnComponentEndOverlap`
  (params (OverlappedComponent :type "PrimitiveComponent Object Reference") (OtherActor :type "Actor Object Reference") (OtherComp :type "PrimitiveComponent Object Reference") (OtherBodyIndex :type Integer))
  ;[0.5569 0.749 1] Specific collision for this event object
  (cast `/Game/Blueprints/FirstPersonCharacter` OtherActor)
  (bind _foundwidgets (`WidgetBlueprintLibrary.GetAllWidgetsOfClass` "/Game/Blueprints/UI/PlayerUI.PlayerUI_C"))
  (`/Game/Blueprints/UI/PlayerUI.ShowInteractAdvice` (`|GetArrayItem` _foundwidgets) false)
  (set `self.isOverlapping?` false))

(fn `UserConstructionScript`
  (`parent.UserConstructionScript`))