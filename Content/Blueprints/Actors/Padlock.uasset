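; Padlock actor that plays an unlock animation when a key is inserted, then drops away as a physics object.
; The Open event runs chained timelines: the first raises the shackle, which then attaches to the body mesh keeping its world transform.
; The second slides the whole actor along world X between hardcoded coordinates, tying it to one level placement, before enabling physics simulation on the body.
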(event `Open`
  (bind (_returnvalue_x _returnvalue_y _returnvalue_z) (`KismetMathLibrary.BreakVector` (`self.K2_GetActorLocation`)))
  (bind _shackle (`self.shackle`))
  (bind (_relativelocation_x _relativelocation_y) (`KismetMathLibrary.BreakVector` (`SceneComponent.RelativeLocation` _shackle)))
  ;[0.7412 0.1843 0] Play padlock animation at insert a key
  (bind (_direction _alpha) (`Timeline|ShackleToUp`)
    (:`Update`
      (`SceneComponent.K2_SetRelativeLocation` _shackle (`KismetMathLibrary.MakeVector` _relativelocation_x _relativelocation_y (`KismetMathLibrary.Lerp` 7.0 9.5 _alpha)) false false))
    (:`Finished`
      (`SceneComponent.K2_AttachToComponent` (`self.shackle`) (`self.StaticMesh`) "None" "KeepWorld" "KeepWorld" "KeepWorld" true)
      (bind (_direction_2 _alpha_2) (`Timeline|PadlockOut`)
        (:`Update`
          (`self.K2_SetActorLocation` (`KismetMathLibrary.MakeVector` (`KismetMathLibrary.Lerp` -9774.9375 -9660.510742 _alpha_2) _returnvalue_y _returnvalue_z)))
        (:`Finished`
          (`PrimitiveComponent.SetSimulatePhysics` (`self.StaticMesh`) true))))))

(fn `UserConstructionScript`)