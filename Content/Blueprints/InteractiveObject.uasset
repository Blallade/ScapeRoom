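; Interactive object Blueprint that shows an interact prompt on the player's UI while the FirstPersonCharacter is inside its Col collision.
; Begin and end overlap events toggle the PlayerUI advice and track the state in IsOverlapping.
; ShowIfOverlap lets the prompt be set on demand only while overlapping, returning that widget.
; The UI is found each time through a top-level widget class search, with no interaction action defined here.
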(event `self.Col.OnComponentBeginOverlap`
  (params (OverlappedComponent :type "PrimitiveComponent Object Reference") (OtherActor :type "Actor Object Reference") (OtherComp :type "PrimitiveComponent Object Reference") (OtherBodyIndex :type Integer) (bFromSweep :type Boolean) (SweepResult :type "HitResult Structure (by ref)"))
  (cast `/Game/Blueprints/FirstPersonCharacter` OtherActor)
  (bind _foundwidgets (`WidgetBlueprintLibrary.GetAllWidgetsOfClass` "/Game/Blueprints/UI/PlayerUI.PlayerUI_C"))
  (`/Game/Blueprints/UI/PlayerUI.ShowInteractAdvice` (`|GetArrayItem` _foundwidgets) true)
  (set `self.isOverlapping?` true))

(event `self.Col.OnComponentEndOverlap`
  (params (OverlappedComponent :type "PrimitiveComponent Object Reference") (OtherActor :type "Actor Object Reference") (OtherComp :type "PrimitiveComponent Object Reference") (OtherBodyIndex :type Integer))
  (cast `/Game/Blueprints/FirstPersonCharacter` OtherActor)
  (bind _foundwidgets (`WidgetBlueprintLibrary.GetAllWidgetsOfClass` "/Game/Blueprints/UI/PlayerUI.PlayerUI_C"))
  (`/Game/Blueprints/UI/PlayerUI.ShowInteractAdvice` (`|GetArrayItem` _foundwidgets) false)
  (set `self.isOverlapping?` false))

(fn `ShowIfOverlap`
  (params (`IsActive?` :type Boolean))
  (returns (UI :type "/Game/Blueprints/UI/PlayerUI Object Reference"))
  (if (`self.isOverlapping?`)
    (bind _foundwidgets (`WidgetBlueprintLibrary.GetAllWidgetsOfClass` "/Game/Blueprints/UI/PlayerUI.PlayerUI_C"))
    (bind _output (`|GetArrayItem` _foundwidgets))
    (`/Game/Blueprints/UI/PlayerUI.ShowInteractAdvice` _output `IsActive?`)
    (return _output)))

(fn `UserConstructionScript`)