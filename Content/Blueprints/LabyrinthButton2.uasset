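; Labyrinth button that, when interacted with, opens the way by destroying MazeOutCenterCheckDoor2 with a rock-crash sound at its location.
; It hides the mouse cursor, removes its own Col component and plays a timeline that adds its value to the button's current X position on each update.
; When the timeline finishes, it calls Return on the PlayerUI widget and has MazeFinalButton run ButtonsChecker.
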(event `/Game/Blueprints/InteractiveEvent.InteractiveEvent`
  (params (Object :type "Actor Object Reference"))
  (bind (_returnvalue_x _returnvalue_y _returnvalue_z) (`KismetMathLibrary.BreakVector` (`self.K2_GetActorLocation`)))
  (set `PlayerController.bShowMouseCursor` false (`GameplayStatics.GetPlayerController` 0))
  (bind _returnvalue (`GameplayStatics.GetActorOfClass` "/Game/Blueprints/Actors/MazeOutCenterCheckDoor2.MazeOutCenterCheckDoor2_C"))
  (`GameplayStatics.SpawnSoundAtLocation` "/Game/Audio/SoundFx/Rocas_chocando.Rocas_chocando" (`self.K2_GetActorLocation` _returnvalue) (struct) 0.2 1.0 0.0 null null)
  (`self.K2_DestroyActor` _returnvalue)
  (`ActorComponent.K2_DestroyComponent` (`self.Col`))
  (bind (_direction _value) (`Timeline|Timeline_0`)
    (:`Update`
      (`self.K2_SetActorLocation` (`KismetMathLibrary.MakeVector` (+ _value _returnvalue_x) _returnvalue_y _returnvalue_z)))
    (:`Finished`
      (bind _foundwidgets (`WidgetBlueprintLibrary.GetAllWidgetsOfClass` "/Game/Blueprints/UI/PlayerUI.PlayerUI_C"))
      (`/Game/Blueprints/UI/PlayerUI.Return` (`|GetArrayItem` _foundwidgets) Object)
      (bind _returnvalue_2 (`GameplayStatics.GetActorOfClass` "/Game/Blueprints/MazeFinalButton.MazeFinalButton_C"))
      (`/Game/Blueprints/MazeFinalButton.ButtonsChecker` _returnvalue_2))))

(fn `UserConstructionScript`)