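; Music manager actor that crossfades between the main theme and the labyrinth horror ambience as the first-person character moves between areas.
; BeginPlay spawns both 2D sounds, leaving the labyrinth one inactive.
; LabyrinthCol and RoomCol overlaps drive two DoOnce gates that re-arm each other, so switches alternate.
; ToggleThemes fades the new track in, while StopTheme fades the old one out and deactivates it after a delay.
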(event `self.ReceiveBeginPlay`
  ;[1 1 1] Begin play set-up
  (bind _returnvalue (`GameplayStatics.SpawnSound2D` "/Game/Audio/Intro_Main_BSO_Scape_Room.Intro_Main_BSO_Scape_Room" 1.0 1.0 0.0 null false false))
  (set `self.main Theme` _returnvalue)
  (bind _returnvalue_2 (`GameplayStatics.SpawnSound2D` "/Game/Audio/Ambience_horror.Ambience_horror" 1.0 1.0 0.0 null false false))
  (bind _output_get (set `self.labirynth Theme` _returnvalue_2))
  (`ActorComponent.SetActive` _output_get false false))

(event `ToggleThemes`
  (params (audioToPlay :type "AudioComponent Object Reference") (audioToStop :type "AudioComponent Object Reference"))
  ;[0.5294 0.0549 0.4902] Toggles between given audios with fades
  (`self.StopTheme` audioToStop)
  (`ActorComponent.SetActive` audioToPlay true false)
  (`AudioComponent.FadeIn` audioToPlay 2.0 1.0 0.0 "Linear"))

(event `StopTheme`
  (params (audioToStop :type "AudioComponent Object Reference"))
  ;[0.5294 0.0549 0.4902] Stops the given audio with a fade out
  (`AudioComponent.FadeOut` audioToStop 2.0 0.0 "Linear")
  (`KismetSystemLibrary.Delay` 2.0)
  (`ActorComponent.SetActive` audioToStop false false))

(event `self.LabyrinthCol.OnComponentBeginOverlap`
  (params (OverlappedComponent :type "PrimitiveComponent Object Reference") (OtherActor :type "Actor Object Reference") (OtherComp :type "PrimitiveComponent Object Reference") (OtherBodyIndex :type Integer) (bFromSweep :type Boolean) (SweepResult :type "HitResult Structure (by ref)"))
  ;[0.2866 1 0.1979] Collisions that switch the audios
  (`/Engine/EditorBlueprintResources/StandardMacros.DoOnce` false :!label _label
    (:`Completed`
      (cast `/Game/Blueprints/FirstPersonCharacter` OtherActor)
      (`self.ToggleThemes` (`self.labirynth Theme`) (`self.main Theme`))
      (goto _label_2 :!via `Reset`))))

(event `self.RoomCol.OnComponentBeginOverlap`
  (params (OverlappedComponent :type "PrimitiveComponent Object Reference") (OtherActor :type "Actor Object Reference") (OtherComp :type "PrimitiveComponent Object Reference") (OtherBodyIndex :type Integer) (bFromSweep :type Boolean) (SweepResult :type "HitResult Structure (by ref)"))
  ;[0.2866 1 0.1979] Collisions that switch the audios
  (`/Engine/EditorBlueprintResources/StandardMacros.DoOnce` true :!label _label_2
    (:`Completed`
      (cast `/Game/Blueprints/FirstPersonCharacter` OtherActor)
      (`self.ToggleThemes` (`self.main Theme`) (`self.labirynth Theme`))
      (goto _label :!via `Reset`))))

(fn `UserConstructionScript`)