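; KeyShelf is a shelf actor that slides aside with its key when the player completes the slider puzzle.
; SlideKeyShelf finds the SliderPuzzleKey actor, enables query-only collision on it, then snaps shelf and key to their start positions.
; The AlphaLerp timeline then lerps both between hardcoded world coordinates, moving the shelf along Y and driving the key through MoveKey.
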(event `SlideKeyShelf`
  (bind (_returnvalue_x _returnvalue_y _returnvalue_z) (`KismetMathLibrary.BreakVector` (`SceneComponent.K2_GetComponentLocation` (`self.StaticMeshComponent`))))
  ;[0.1175 1 0.1248] Slides the Keyshelf when player completes the slider puzzle and enable the key collision
  (bind _returnvalue (`GameplayStatics.GetActorOfClass` "/Game/Blueprints/SliderPuzzleKey.SliderPuzzleKey_C"))
  (`PrimitiveComponent.SetCollisionEnabled` (`/Game/Blueprints/InteractiveObject.Col` _returnvalue) "QueryOnly")
  (`/Game/Blueprints/SliderPuzzleKey.MoveKey` _returnvalue 9693.205078)
  (`self.K2_SetActorLocation` (`KismetMathLibrary.MakeVector` _returnvalue_x 10241.205078 _returnvalue_z))
  (bind (_direction _newtrack_0) (`Timeline|AlphaLerp`)
    (:`Update`
      (`self.K2_SetActorLocation` (`KismetMathLibrary.MakeVector` _returnvalue_x (`KismetMathLibrary.Lerp` 10241.205078 9999.205078 _newtrack_0) _returnvalue_z))
      (`/Game/Blueprints/SliderPuzzleKey.MoveKey` _returnvalue (`KismetMathLibrary.Lerp` 9693.205078 9451.205078 _newtrack_0)))))

(fn `UserConstructionScript`)