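; SliderTable is an interactive actor that serves as the in-world entry point to a slider puzzle.
; InteractiveEvent switches the FirstPersonCharacter to its puzzle camera, waits briefly, then shows the back button on the SliderPuzzleUI widget and enables input on itself.
; The BackKey action calls PressBackKey on the first SliderPuzzleUI found and disables the actor's input again.
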(event `/Game/Blueprints/InteractiveEvent.InteractiveEvent`
  (params (Object :type "Actor Object Reference"))
  (`/Game/Blueprints/FirstPersonCharacter.ChangesCameraAtPuzzle` (cast `/Game/Blueprints/FirstPersonCharacter` (`GameplayStatics.GetPlayerCharacter` 0) :!pure true) true)
  (bind _foundwidgets (`WidgetBlueprintLibrary.GetAllWidgetsOfClass` "/Game/Blueprints/UI/SliderPuzzleUI.SliderPuzzleUI_C"))
  (`KismetSystemLibrary.Delay` 1.0)
  (`/Game/Blueprints/UI/SliderPuzzleUI.ShowBackButton` _foundwidgets Object)
  (`self.EnableInput` (`GameplayStatics.GetPlayerController` 0)))

(event `InputAction|BackKey`
  (params (Key :type "Key Structure"))
  (:`Pressed`
    (bind _foundwidgets (`WidgetBlueprintLibrary.GetAllWidgetsOfClass` "/Game/Blueprints/UI/SliderPuzzleUI.SliderPuzzleUI_C"))
    (`/Game/Blueprints/UI/SliderPuzzleUI.PressBackKey` (`|GetArrayItem` _foundwidgets))
    (`self.DisableInput` (`GameplayStatics.GetPlayerController` 0))))

(fn `UserConstructionScript`)