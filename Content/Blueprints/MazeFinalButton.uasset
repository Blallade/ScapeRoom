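; Final button of the maze puzzle, which opens the way out and unlocks the labyrinth key.
; A button counter destroys the center wall with a rock sound once enough checks accumulate.
; Interacting removes the button's collider, cell bars, exit wall and exit door, then a timeline sinks the button.
; When it finishes, the key's collision becomes query-only, a checkpoint sound plays and the player UI is notified.
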(event `/Game/Blueprints/InteractiveEvent.InteractiveEvent`
  (params (Object :type "Actor Object Reference"))
  (bind (_returnvalue_x _returnvalue_y _returnvalue_z) (`KismetMathLibrary.BreakVector` (`self.K2_GetActorLocation`)))
  ;[0.7098 0.1647 0.698] Push the final button and unlock the key
  (set `PlayerController.bShowMouseCursor` false (`GameplayStatics.GetPlayerController` 0))
  (`ActorComponent.K2_DestroyComponent` (`self.Col`))
  (bind _returnvalue (`GameplayStatics.GetActorOfClass` "/Game/Blueprints/Actors/CellBars.CellBars_C"))
  (bind _returnvalue_2 (`GameplayStatics.GetActorOfClass` "/Game/Blueprints/Actors/MazeCenterExitWall.MazeCenterExitWall_C"))
  (bind _returnvalue_3 (`GameplayStatics.GetActorOfClass` "/Game/Blueprints/Actors/MazeOutCenterExitDoor.MazeOutCenterExitDoor_C"))
  (`GameplayStatics.SpawnSoundAtLocation` "/Game/Audio/SoundFx/Rocas_chocando.Rocas_chocando" (`self.K2_GetActorLocation` _returnvalue_3) (struct) 0.2 1.3 0.0 null null)
  (`self.K2_DestroyActor` _returnvalue_2)
  (`self.K2_DestroyActor` _returnvalue_3)
  (`self.K2_DestroyActor` _returnvalue)
  (bind (_direction _value) (`Timeline|Timeline_0`)
    (:`Update`
      (`self.K2_SetActorLocation` (`KismetMathLibrary.MakeVector` _returnvalue_x _returnvalue_y (- _returnvalue_z _value))))
    (:`Finished`
      (bind _returnvalue_4 (`GameplayStatics.GetActorOfClass` "/Game/Blueprints/LabyrinthKey.LabyrinthKey_C"))
      (`PrimitiveComponent.SetCollisionEnabled` (`/Game/Blueprints/InteractiveObject.Col` _returnvalue_4) "QueryOnly")
      (`GameplayStatics.PlaySound2D` "/Game/Audio/SoundFx/Checkpoint.Checkpoint" 1.0 1.0 0.0 null null)
      (bind _foundwidgets (`WidgetBlueprintLibrary.GetAllWidgetsOfClass` "/Game/Blueprints/UI/PlayerUI.PlayerUI_C"))
      (`/Game/Blueprints/UI/PlayerUI.Return` (`|GetArrayItem` _foundwidgets) Object))))

(event `ButtonsChecker`
  ;[0.4844 0.05046 0.08879] Checks the number of buttons pressed
  (if (>= (`self.ButtonsCheck`) 2)
    (bind _returnvalue (`GameplayStatics.GetActorOfClass` "/Game/Blueprints/Actors/MazeCenterWall.MazeCenterWall_C"))
    (`GameplayStatics.SpawnSoundAtLocation` "/Game/Audio/SoundFx/Rocas_chocando.Rocas_chocando" (`self.K2_GetActorLocation` _returnvalue) (struct) 0.2 1.3 0.0 null null)
    (`self.K2_DestroyActor` _returnvalue)
    (else
      (set `self.ButtonsCheck` (+ (`self.ButtonsCheck`) 1)))))

(fn `UserConstructionScript`
  (`parent.UserConstructionScript`))