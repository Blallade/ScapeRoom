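; Padlocked double door that consumes a held key per interaction to open padlocks, and swings open on an interaction once three are unlocked.
; Without a key it shows a DoorUI warning, using any held item except the magnifying glass as one.
; Timelines rotate two pivots in mirrored directions.
; When the player overlaps Col1, the door closes, then once stops the main theme and starts the outro UI animation.
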(event `self.Col1.OnComponentBeginOverlap`
  (params (OverlappedComponent :type "PrimitiveComponent Object Reference") (OtherActor :type "Actor Object Reference") (OtherComp :type "PrimitiveComponent Object Reference") (OtherBodyIndex :type Integer) (bFromSweep :type Boolean) (SweepResult :type "HitResult Structure (by ref)"))
  (bind _pivot1 (`self.pivot1`))
  (bind (_returnvalue_roll _returnvalue_pitch _returnvalue_yaw) (`KismetMathLibrary.BreakRotator` (`SceneComponent.K2_GetComponentRotation` _pivot1)))
  ;[1 0.3176 0.1451] Closes the door
  (`|ExecutionSequence`
    (:`then_0`
      (cast `/Game/Blueprints/FirstPersonCharacter` OtherActor)
      (bind (_direction _alpha) (`Timeline|CloseDoor`)
        (:`Update`
          (bind _returnvalue (`KismetMathLibrary.Lerp` (`self.newRotation`) 0.0 _alpha))
          (`SceneComponent.K2_SetWorldRotation` (`self.pivot1`) (`KismetMathLibrary.MakeRotator` 0.0 0.0 _returnvalue) false false)
          (`SceneComponent.K2_SetWorldRotation` (`self.pivot2`) (`KismetMathLibrary.MakeRotator` 0.0 0.0 (* _returnvalue -1.0)) false false))
        (:`Finished`
          (`/Engine/EditorBlueprintResources/StandardMacros.DoOnce` false
            (:`Completed`
              (`GameplayStatics.PlaySound2D` "/Game/Audio/SoundFx/Puerta_cerrando.Puerta_cerrando" 10.0 1.2 0.1 null null)
              (bind _returnvalue_2 (`GameplayStatics.GetActorOfClass` "/Game/Blueprints/MusicManager.MusicManager_C"))
              (`/Game/Blueprints/MusicManager.StopTheme` _returnvalue_2 (`/Game/Blueprints/MusicManager.main Theme` _returnvalue_2))
              (bind _foundwidgets (`WidgetBlueprintLibrary.GetAllWidgetsOfClass` "/Game/Blueprints/UI/OutroUI.OutroUI_C"))
              (bind _output (`|GetArrayItem` _foundwidgets))
              (`WidgetBlueprintLibrary.SetInputMode_UIOnlyEx` (`GameplayStatics.GetPlayerController` 0) _output)
              (bind _returnvalue_3 (`GameplayStatics.GetActorOfClass` "/Game/Blueprints/FirstPersonCharacter.FirstPersonCharacter_C"))
              (set `/Game/Blueprints/FirstPersonCharacter.Targetting` true _returnvalue_3)
              (`/Game/Blueprints/UI/OutroUI.FinalAnimation` _output))))))
    (:`then_1`
      ;[1 0.3176 0.1451] Opens the door
      (bind (_direction_2 _alpha_2) (`Timeline|OpenDoor` :!via `Stop` :!label _label)
        (:`Update`
          (bind _returnvalue_4 (`KismetMathLibrary.Lerp` _returnvalue_yaw (`self.newRotation`) _alpha_2))
          (`SceneComponent.K2_SetWorldRotation` _pivot1 (`KismetMathLibrary.MakeRotator` 0.0 0.0 _returnvalue_4) false false)
          (`SceneComponent.K2_SetWorldRotation` (`self.pivot2`) (`KismetMathLibrary.MakeRotator` 0.0 0.0 (* _returnvalue_4 -1.0)) false false))))))

(event `/Game/Blueprints/InteractiveEvent.InteractiveEvent`
  (params (Object :type "Actor Object Reference"))
  ;[0.6196 0.1098 0.1098] Checks the number of padlocks open
  (`PrimitiveComponent.SetCollisionEnabled` (`self.Col`) "NoCollision")
  (if (>= (`self.PadlocksOpen`) 3)
    ;[1 0.2275 0.9804] Allow the character to move
    (`self.DisableInput` (`GameplayStatics.GetPlayerController` 0))
    (bind _foundwidgets (`WidgetBlueprintLibrary.GetAllWidgetsOfClass` "/Game/Blueprints/UI/PlayerUI.PlayerUI_C"))
    (`/Game/Blueprints/UI/PlayerUI.Return` (`|GetArrayItem` _foundwidgets) self)
    ;[1 0.3176 0.1451] Opens the door
    (`GameplayStatics.PlaySound2D` "/Game/Audio/SoundFx/Checkpoint.Checkpoint" 1.0 1.0 0.0 null null)
    (goto _label)
    (else
      ;[0.3802 0.3782 0.3782] Finds a key in the player hands
      (`self.EnableInput` (`GameplayStatics.GetPlayerController` 0))
      (bind _values (`BlueprintMapLibrary.Map_Values` (`/Game/Blueprints/FirstPersonCharacter.HandsObjects` (cast `/Game/Blueprints/FirstPersonCharacter` (`GameplayStatics.GetPlayerCharacter` 0) :!pure true))))
      (for _index (range 2)
        (bind _output (`|GetArrayItem` _values _index))
        (`/Engine/EditorBlueprintResources/StandardMacros.IsValid` _output
          (:`Is Valid`
            (if (!= (`GameplayStatics.GetObjectClass` _output) "/Game/Blueprints/MagnifyingGlass.MagnifyingGlass_C")
              (set `self.key` _output)
              (set `self.keyFound?` true)
              (break)))))
      ;[0.599 0.05615 0.05615] Checks if the player has a key
      (if (`self.keyFound?`)
        (set `self.keyFound?` false)
        ;[1 0.2275 0.9804] Allow the character to move
        (`self.DisableInput` (`GameplayStatics.GetPlayerController` 0))
        (bind _foundwidgets_2 (`WidgetBlueprintLibrary.GetAllWidgetsOfClass` "/Game/Blueprints/UI/PlayerUI.PlayerUI_C"))
        (`/Game/Blueprints/UI/PlayerUI.Return` (`|GetArrayItem` _foundwidgets_2) self)
        ;[1 0.3176 0.1451] Opens the padlock
        (bind _outactors (`GameplayStatics.GetAllActorsOfClass` "/Game/Blueprints/Actors/Padlock.Padlock_C"))
        (`/Game/Blueprints/Actors/Padlock.Open` (`|GetArrayItem` _outactors (`self.PadlocksOpen`)))
        (`/Game/Blueprints/FirstPersonCharacter.ClearObject` (cast `/Game/Blueprints/FirstPersonCharacter` (`GameplayStatics.GetPlayerCharacter` 0) :!pure true) (`self.key`))
        (`KismetSystemLibrary.Delay` 2.2)
        (bind _result (`/Engine/EditorBlueprintResources/StandardMacros.IncrementInt` (`self.PadlocksOpen`))
          (:`  `
            (set `self.PadlocksOpen` _result)
            (`PrimitiveComponent.SetCollisionEnabled` (`self.Col`) "QueryOnly")))
        (else
          ;[1 0.8427 0.06105] Shows the player the "no key" advice
          (bind _foundwidgets_3 (`WidgetBlueprintLibrary.GetAllWidgetsOfClass` "/Game/Blueprints/UI/DoorUI.DoorUI_C"))
          (`/Game/Blueprints/UI/DoorUI.ShowNoKeyAdvice` (`|GetArrayItem` _foundwidgets_3) true self))))))

(event `PressConfirmInteraction`
  ;[0.5156 0.09199 0.4497] Disable input
  (`self.DisableInput` (`GameplayStatics.GetPlayerController` 0))
  (`PrimitiveComponent.SetCollisionEnabled` (`self.Col`) "QueryOnly"))

(event `InputAction|Continue`
  (params (Key :type "Key Structure"))
  ;[0.05673 0.9003 1] Press "E" interaction
  (:`Pressed`
    (bind _foundwidgets (`WidgetBlueprintLibrary.GetAllWidgetsOfClass` "/Game/Blueprints/UI/DoorUI.DoorUI_C"))
    (`/Game/Blueprints/UI/DoorUI.PressEKey` (`|GetArrayItem` _foundwidgets))))

(fn `UserConstructionScript`
  (`parent.UserConstructionScript`))