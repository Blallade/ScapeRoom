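; Sliding tile puzzle actor that opens the key shelf and exits the puzzle camera and UI when solved.
; Construction builds a scaled grid of box slots and textured tiles, optionally shuffled with an inversion-parity fix to keep it solvable.
; Clicking a tile sphere-searches nearby slots for an unoccupied one and slides there on a timeline, blocking clicks meanwhile.
; After each move, overlaps between tiles and their home slots determine completion.
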(event `self.ReceiveBeginPlay`
  (for _array_element (`self.meshesList`)
    (add `PrimitiveComponent.OnClicked` _array_element (delegate `MeshClicked`))))

(event `MeshClicked`
  (params (TouchedComponent :type "PrimitiveComponent Object Reference") (ButtonPressed :type "Key Structure"))
  (bind _output_get (set `self.ClickedMesh` TouchedComponent))
  (add `PrimitiveComponent.OnClicked` _output_get (delegate `MeshClicked`))
  (bind _neighbors (`self.GetNeighbors`))
  (`self.GetMoveTo` _neighbors)
  (`/Engine/EditorBlueprintResources/StandardMacros.IsValid` (`self.moveToTarget`)
    (:`Is Valid`
      (`self.MoveTo`))))

(event `MoveTo`
  (set `PlayerController.bEnableClickEvents` false (`GameplayStatics.GetPlayerController` 0))
  (set `self.moveToStart` (`SceneComponent.RelativeLocation` (`self.ClickedMesh`)))
  (`GameplayStatics.PlaySound2D` "/Game/Audio/SoundFx/Deslizamiento_papel_mesa.Deslizamiento_papel_mesa" 1.0 1.0 0.1 null null)
  (bind (_direction _newtrack_0) (`Timeline|Timeline_0` :!via `PlayFromStart`)
    (:`Update`
      (`SceneComponent.K2_SetRelativeLocation` (`self.ClickedMesh`) (`KismetMathLibrary.VLerp` (`self.moveToStart`) (`SceneComponent.RelativeLocation` (`self.moveToTarget`)) _newtrack_0) false false))
    (:`Finished`
      (set `PlayerController.bEnableClickEvents` true (`GameplayStatics.GetPlayerController` 0))
      (bind _solved (`self.IsSolved?`))
      (if _solved
        (`/Engine/EditorBlueprintResources/StandardMacros.DoOnce` false
          (:`Completed`
            (`self.PuzzleSolved!`)))))))

(fn `GetMoveTo`
  (params (neighborsList :type "Array of PrimitiveComponent Object Reference"))
  (set `self.moveToTarget` null)
  (for _array_element neighborsList
    (if (not (`PrimitiveComponent.IsOverlappingActor` _array_element self))
      (set `self.moveToTarget` _array_element)))
  (return))

(fn `GetNeighbors`
  (returns (neighbors :type "Array of PrimitiveComponent Object Reference"))
  (bind _returnvalue (`GameplayStatics.GetActorOfClass` "/Game/Blueprints/SliderTable.SliderTable_C"))
  (bind _outcomponents (`KismetSystemLibrary.SphereOverlapComponents` (`SceneComponent.K2_GetComponentLocation` (`self.ClickedMesh`)) (* (`self.meshSize`) 3.0) (`|MakeArray` "ObjectTypeQuery1" "ObjectTypeQuery2" :!type "EObjectTypeQuery Enum") "/Script/Engine.BoxComponent" (`|MakeArray` _returnvalue :!type "Actor Object Reference")))
  (return _outcomponents))

(fn `IsSolved?`
  (returns (solved :type Boolean))
  (locals (solve :type Boolean :default true))
  (for (_array_element _array_index) (`self.meshesList`)
    (if (not (`PrimitiveComponent.IsOverlappingComponent` _array_element (`|GetArrayItem` (`self.spaceList`) _array_index)))
      (set `local.solve` false)
      (break)))
  (return (`local.solve`)))

(fn `PuzzleSolved!`
  (`GameplayStatics.PlaySound2D` "/Game/Audio/SoundFx/Checkpoint.Checkpoint" 1.0 1.0 0.0 null null)
  (`/Game/Blueprints/FirstPersonCharacter.ChangesCameraAtPuzzle` (cast `/Game/Blueprints/FirstPersonCharacter` (`GameplayStatics.GetPlayerCharacter` 0) :!pure true) false)
  (bind _foundwidgets (`WidgetBlueprintLibrary.GetAllWidgetsOfClass` "/Game/Blueprints/UI/SliderPuzzleUI.SliderPuzzleUI_C"))
  (`/Game/Blueprints/UI/SliderPuzzleUI.PressBackKey` (`|GetArrayItem` _foundwidgets))
  (`self.DisableInput` null)
  (bind _returnvalue (`GameplayStatics.GetActorOfClass` "/Game/Blueprints/SliderTable.SliderTable_C"))
  (`self.DisableInput` _returnvalue (`GameplayStatics.GetPlayerController` 0))
  (bind _outactors (`GameplayStatics.GetAllActorsOfClass` "/Game/Blueprints/KeyShelf.KeyShelf_C"))
  (`/Game/Blueprints/KeyShelf.SlideKeyShelf` (`|GetArrayItem` _outactors)))

(fn `ScalePuzzle`
  (`self.SetActorScale3D` (/ (1.0 1.0 0.3) (/ (* (`self.gridSize`) (`self.meshSize`)) (`self.desiredSize`))))
  (return))

(fn `ShuffleMeshes`
  (for _array_element (`self.spaceList`)
    (`KismetArrayLibrary.Array_Add` (`self.location`) (`SceneComponent.RelativeLocation` _array_element)))
  (for (_array_element_2 _array_index) (`self.location`)
    (`SceneComponent.K2_SetRelativeLocation` (`|GetArrayItem` (`self.meshesList`) (`|GetArrayItem` (`self.combinationList`) _array_index)) _array_element_2 false false))
  (`KismetArrayLibrary.Array_Clear` (`self.location`)))

(fn `ShufflePuzzle`
  (locals (emptySlot :type Integer :default 8) (numberOfInversions :type Integer) (i :type Integer))
  (bind _combinationlist (`self.combinationList`))
  (bind _emptyslot (`local.emptySlot`))
  (bind _combinationlist_2 (`self.combinationList`))
  (bind _emptyslot_2 (`local.emptySlot`))
  (bind _emptyslot_3 (`local.emptySlot`))
  (bind _combinationlist_3 (`self.combinationList`))
  (bind _combinationlist_4 (`self.combinationList`))
  (bind _combinationlist_5 (`self.combinationList`))
  (bind _returnvalue (`KismetArrayLibrary.Array_LastIndex` _combinationlist_5))
  (bind _returnvalue_2 (- (`self.gridSize`) 1))
  (bind _returnvalue_3 (* (`self.gridSize`) (`self.gridSize`)))
  (bind _returnvalue_4 (* (`self.gridSize`) (`self.gridSize`)))
  (bind _returnvalue_5 (* (`self.gridSize`) (`self.gridSize`)))
  (set `local.emptySlot` (- (* (`self.gridSize`) (`self.gridSize`)) 1))
  (`KismetArrayLibrary.Array_Shuffle` _combinationlist_5)
  (for _index (range (+ _returnvalue 1))
    (set `local.i` _index)
    (if (not (== (`|GetArrayItem` (`self.combinationList`) _index) (`local.emptySlot`)))
      (for _index_2 (range (+ (`local.i`) 1) (+ _returnvalue 1))
        (bind _output (`|GetArrayItem` _combinationlist _index_2))
        (if (and (!= _output (`local.emptySlot`)) (< _output (`|GetArrayItem` _combinationlist (`local.i`))))
          (`/Engine/EditorBlueprintResources/StandardMacros.IncrementInt` (`local.numberOfInversions`))))))
  (if (!= (mod (`self.gridSize`) 2) 0)
    (if (!= (mod (`local.numberOfInversions`) 2) 0)
      (if (and (!= (`|GetArrayItem` (`self.combinationList`)) _emptyslot) (!= _emptyslot (`|GetArrayItem` (`self.combinationList`) 1)))
        (`KismetArrayLibrary.Array_Swap` _combinationlist_2 0 1)
        (else
          (`KismetArrayLibrary.Array_Swap` _combinationlist_2 (- _returnvalue_3 1) (- _returnvalue_3 2))))
      (`self.ShuffleMeshes`)
      (else
        (`self.ShuffleMeshes`)))
    (else
      (for _index_3 (range (+ _returnvalue_2 1))
        (for _index_4 (range (+ _returnvalue_2 1))
          (`BlueprintMapLibrary.Map_Add` (`self.combinationRowsList`) (`|GetArrayItem` (`self.combinationList`) (+ (* _index_3 (`self.gridSize`)) _index_4)) _index_3)))
      (if (!= (mod (`BlueprintMapLibrary.Map_Find` (`self.combinationRowsList`) (`local.emptySlot`)) 2) 0)
        (if (!= (mod (`local.numberOfInversions`) 2) 0)
          (if (and (!= (`|GetArrayItem` (`self.combinationList`)) _emptyslot_3) (!= _emptyslot_3 (`|GetArrayItem` (`self.combinationList`) 1)))
            (`KismetArrayLibrary.Array_Swap` _combinationlist_3 0 1)
            (else
              (`KismetArrayLibrary.Array_Swap` _combinationlist_3 (- _returnvalue_4 1) (- _returnvalue_4 2))))
          (`self.ShuffleMeshes`)
          (else
            (`self.ShuffleMeshes`)))
        (elif (== (mod (`local.numberOfInversions`) 2) 0)
          (if (and (!= (`|GetArrayItem` (`self.combinationList`)) _emptyslot_2) (!= _emptyslot_2 (`|GetArrayItem` (`self.combinationList`) 1)))
            (`KismetArrayLibrary.Array_Swap` _combinationlist_4 0 1)
            (else
              (`KismetArrayLibrary.Array_Swap` _combinationlist_4 (- _returnvalue_5 1) (- _returnvalue_5 2))))
          (`self.ShuffleMeshes`)
          (else
            (`self.ShuffleMeshes`)))))))

(fn `SpawnPuzzle`
  (bind _meshsize (`self.meshSize`))
  (bind _spacelist (`self.spaceList`))
  (bind _mesheslist (`self.meshesList`))
  (bind _meshsize_2 (`self.meshSize`))
  (bind _returnvalue (- (`self.gridSize`) 1))
  (bind _returnvalue_2 (/ (`self.meshSize`) 4.0))
  (bind _returnvalue_3 (- (`self.gridSize`) 1))
  (`KismetArrayLibrary.Array_Clear` (`self.combinationList`))
  (bind (_arrayindex _arrayelement) (`/Engine/EditorBlueprintResources/StandardMacros.ReverseForEachLoop` _spacelist)
    (:`LoopBody`
      (`ActorComponent.K2_DestroyComponent` _arrayelement))
    (:`Completed`
      (`KismetArrayLibrary.Array_Clear` _spacelist)
      (bind (_arrayindex_2 _arrayelement_2) (`/Engine/EditorBlueprintResources/StandardMacros.ReverseForEachLoop` _mesheslist)
        (:`LoopBody`
          (`ActorComponent.K2_DestroyComponent` _arrayelement_2))
        (:`Completed`
          (`KismetArrayLibrary.Array_Clear` _mesheslist)
          (for _index (range (+ _returnvalue 1))
            (set `self.Y Index` _index)
            (for _index_2 (range (+ _returnvalue 1))
              (set `self.X Index` _index_2)
              (`KismetArrayLibrary.Array_Add` (`self.combinationList`) (+ (* (`self.Y Index`) (`self.gridSize`)) (`self.X Index`)))
              (bind _returnvalue_4 (`AddComponent|NODE_AddBoxComponent-0` :`RelativeTransform` (`KismetMathLibrary.MakeTransform` (`KismetMathLibrary.MakeVector` (* (`self.X Index`) _meshsize) (* (`self.Y Index`) _meshsize)))))
              (`BoxComponent.SetBoxExtent` _returnvalue_4 (`KismetMathLibrary.MakeVector` _returnvalue_2 _returnvalue_2 _returnvalue_2) true)
              (`KismetArrayLibrary.Array_Add` (`self.spaceList`) _returnvalue_4)
              (if (not (and (== (`self.X Index`) _returnvalue_3) (== _returnvalue_3 (`self.Y Index`))))
                (bind _returnvalue_5 (`AddComponent|NODE_AddStaticMeshComponent-0` :`RelativeTransform` (`KismetMathLibrary.MakeTransform` (`KismetMathLibrary.MakeVector` (* (`self.X Index`) _meshsize_2) (* (`self.Y Index`) _meshsize_2)))))
                (`KismetArrayLibrary.Array_Add` (`self.meshesList`) _returnvalue_5)
                (bind _returnvalue_6 (`PrimitiveComponent.CreateDynamicMaterialInstance` _returnvalue_5 0 "/Game/Materials/PuzzleMat.PuzzleMat" "None"))
                (`MaterialInstanceDynamic.SetTextureParameterValue` _returnvalue_6 "PuzzleTexture" (`self.texture`))
                (`MaterialInstanceDynamic.SetScalarParameterValue` _returnvalue_6 "SizeOfGreed" (`KismetMathLibrary.Conv_IntToDouble` (`self.gridSize`)))
                (`MeshComponent.SetVectorParameterValueOnMaterials` _returnvalue_5 "PuzzleCoordinate" (`KismetMathLibrary.MakeVector` (`KismetMathLibrary.Conv_IntToDouble` (`self.X Index`)) (`KismetMathLibrary.Conv_IntToDouble` (`self.Y Index`)))))))
          (return))))))

(fn `UserConstructionScript`
  (`self.SpawnPuzzle`)
  (`self.ScalePuzzle`)
  (if (`self.Shuffle?`)
    (`self.ShufflePuzzle`)))